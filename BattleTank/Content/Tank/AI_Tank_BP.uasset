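; AI tank Blueprint that passes its turret and barrel to the aiming references on BeginPlay.
; Axis inputs rotate the azimuth gimbal, spring arm and camera, and the Fire action calls Fire.
; Tick changes the barrel's minimum elevation by turret yaw to keep it from intersecting the body.
; Any hit on the body destroys the tank's components, leaving the actor itself in place.
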(event `self.ReceiveBeginPlay`
  (`self.SetTurretReference` (`self.TankTurret`))
  (`self.SetBarrelReference` (`self.Barrel`)))

(event `self.Body.OnComponentHit`
  (params (HitComponent :type "PrimitiveComponent Object Reference") (OtherActor :type "Actor Object Reference") (OtherComp :type "PrimitiveComponent Object Reference") (NormalImpulse :type "Vector Structure") (Hit :type "HitResult Structure (by ref)"))
  (`self.deleteComponents`))

(event `InputAxis|AimAzimoth`
  (params (AxisValue :type "Float (single-precision)"))
  ;[1 1 1] Input handling stuff
  (`SceneComponent.K2_AddLocalRotation` (`self.AzimothGimbal`) (`KismetMathLibrary.MakeRotator` 0.0 0.0 (* AxisValue (`GameplayStatics.GetWorldDeltaSeconds`) 70.0)) false false))

(event `InputAxis|AimElevation`
  (params (AxisValue :type "Float (single-precision)"))
  ;[1 1 1] Input handling stuff
  (`SceneComponent.K2_AddLocalRotation` (`self.SpringArm`) (`KismetMathLibrary.MakeRotator` 0.0 (* AxisValue (`GameplayStatics.GetWorldDeltaSeconds`) 70.0)) false false)
  (`SceneComponent.K2_AddLocalRotation` (`self.Camera`) (`KismetMathLibrary.MakeRotator` 0.0 (* AxisValue (`GameplayStatics.GetWorldDeltaSeconds`) 30.0)) false false))

(event `InputAction|Fire`
  (params (Key :type "Key Structure" :default "AnyKey"))
  ;[1 1 1] Input handling stuff
  (:`Pressed`
    (`self.Fire`)))

(event `self.ReceiveTick`
  (params (DeltaSeconds :type "Float (single-precision)"))
  ;[1 1 1] keeps barrel from intersecting tank body
  (if (> (.yaw (`SceneComponent.GetSocketRotation` (`self.TankTurret`) "None")) 40.0)
    (`TankBarrel.SetMinElevation` (`self.Barrel`) 0.0)
    (if (> (.yaw (`SceneComponent.GetSocketRotation` (`self.TankTurret`) "None")) 135.0)
      (`TankBarrel.SetMinElevation` (`self.Barrel`) -10.0)
      (else
        (`TankBarrel.SetMinElevation` (`self.Barrel`) 0.0)))
    (else
      (`TankBarrel.SetMinElevation` (`self.Barrel`) -10.0))))

(fn `UserConstructionScript`)