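; Player-controlled tank pawn that passes its turret and barrel components to setup functions on BeginPlay.
; Input axes rotate the camera gimbal, spring arm and camera for aiming and set track throttles individually or together, while actions fire or reset the tank upright.
; Tick adjusts the barrel's minimum elevation by turret yaw to keep it clear of the body.
; The TankMovementComponent forward-intent call is left unconnected.
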(event `self.ReceiveBeginPlay`
  (`self.SetTurretReference` (`self.TankTurret`))
  (`self.SetBarrelReference` (`self.Barrel`)))

(event `InputAxis|AimAzimoth`
  (params (AxisValue :type "Float (single-precision)"))
  ;[1 1 1] Input handling stuff
  (`SceneComponent.K2_AddLocalRotation` (`self.AzimothGimbal`) (`KismetMathLibrary.MakeRotator` 0.0 0.0 (* AxisValue (`GameplayStatics.GetWorldDeltaSeconds`) 70.0)) false false))

(event `InputAxis|AimElevation`
  (params (AxisValue :type "Float (single-precision)"))
  ;[1 1 1] Input handling stuff
  (`SceneComponent.K2_AddLocalRotation` (`self.SpringArm`) (`KismetMathLibrary.MakeRotator` 0.0 (* AxisValue (`GameplayStatics.GetWorldDeltaSeconds`) 70.0)) false false)
  (`SceneComponent.K2_AddLocalRotation` (`self.Camera`) (`KismetMathLibrary.MakeRotator` 0.0 (* AxisValue (`GameplayStatics.GetWorldDeltaSeconds`) 30.0)) false false))

(event `InputAction|Fire`
  (params (Key :type "Key Structure" :default "AnyKey"))
  ;[1 1 1] Input handling stuff
  (:`Pressed`
    (`self.Fire`)))

(event `InputAction|reset position`
  (params (Key :type "Key Structure" :default "AnyKey"))
  ;[1 1 1] Input handling stuff
  (:`Pressed`
    (`self.K2_SetActorLocationAndRotation` (`KismetMathLibrary.MakeVector` (.x (`self.K2_GetActorLocation`)) (.y (`self.K2_GetActorLocation`)) 5.0) (`KismetMathLibrary.MakeRotator` 0.0 (.pitch (`self.K2_GetActorRotation`)) (.yaw (`self.K2_GetActorRotation`))) true true)))

(event `InputAxis|lefttrackthrottle`
  (params (AxisValue :type "Float (single-precision)"))
  ;[1 1 1] Input handling stuff
  (`TankTracks.SetThrottle` (`self.LeftTrack`) AxisValue))

(event `InputAxis|righttrackthrottle`
  (params (AxisValue :type "Float (single-precision)"))
  ;[1 1 1] Input handling stuff
  (`TankTracks.SetThrottle` (`self.RightTrack`) AxisValue))

(event `InputAxis|Forward`
  (params (AxisValue :type "Float (single-precision)"))
  ;[1 1 1] Input handling stuff
  (`TankTracks.SetThrottle` (`self.LeftTrack`) AxisValue)
  (`TankTracks.SetThrottle` (`self.RightTrack`) AxisValue))

(event `InputAxis|Left Track Reverse`
  (params (AxisValue :type "Float (single-precision)"))
  ;[1 1 1] Input handling stuff
  (`TankTracks.SetThrottle` (`self.LeftTrack`) AxisValue))

(event `InputAxis|backward`
  (params (AxisValue :type "Float (single-precision)"))
  ;[1 1 1] Input handling stuff
  (`TankTracks.SetThrottle` (`self.LeftTrack`) AxisValue)
  (`TankTracks.SetThrottle` (`self.RightTrack`) AxisValue))

(event `InputAxis|Right Track Reverse`
  (params (AxisValue :type "Float (single-precision)"))
  ;[1 1 1] Input handling stuff
  (`TankTracks.SetThrottle` (`self.RightTrack`) AxisValue))

(event `InputAxis|Move Forward`
  (params (AxisValue :type "Float (single-precision)"))
  ;[1 1 1] Input handling stuff
  (`TankTracks.SetThrottle` (`self.LeftTrack`) AxisValue)
  (`TankTracks.SetThrottle` (`self.RightTrack`) AxisValue))

(event `self.ReceiveTick`
  (params (DeltaSeconds :type "Float (single-precision)"))
  ;[1 1 1] keeps barrel from intersecting tank body
  (if (> (.yaw (`SceneComponent.GetSocketRotation` (`self.TankTurret`) "None")) 40.0)
    (`TankBarrel.SetMinElevation` (`self.Barrel`) 0.0)
    (if (> (.yaw (`SceneComponent.GetSocketRotation` (`self.TankTurret`) "None")) 135.0)
      (`TankBarrel.SetMinElevation` (`self.Barrel`) -10.0)
      (else
        (`TankBarrel.SetMinElevation` (`self.Barrel`) 0.0)))
    (else
      (`TankBarrel.SetMinElevation` (`self.Barrel`) -10.0))))

(fn `UserConstructionScript`)